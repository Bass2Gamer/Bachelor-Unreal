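; Damage system component that tracks health and death state for whatever owns it.
; TakeDamage subtracts the amount in a DamageInfo struct from Health, ignores hits once dead, and fires OnDeath when health runs out.
; Surviving hits fire OnDamageResponse with the struct's response type only if the target is interruptible or the hit forces an interrupt.
; It returns true only on death or interrupt.
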(event EventBeginPlay)

(event EventTick
  (params (DeltaSeconds :type Float%20%28single-precision%29)))

(fn TakeDamage
  (params (DamageInfo :type S%20Damage%20Info%20Structure))
  (bind (_amount _damagetype _damageresponse _shouldforceinterrupt) (Utilities|Struct|BreakS_DamageInfo DamageInfo))
  (if (not (Variables|Default|GetIsDead))
    (bind _output_get (Variables|Default|SetHealth (- (Variables|Default|GetHealth) _amount)))
    (if (<= _output_get 0.0)
      (Variables|Default|SetIsDead true)
      (Default|CallOnDeath)
      (return true)
      (elif (or (Variables|Default|GetIsInterruptible) _shouldforceinterrupt)
        (Default|CallOnDamageResponse _damageresponse)
        (return true)))))