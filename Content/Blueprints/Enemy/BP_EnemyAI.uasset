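; Skeleton enemy AI that roams, chases the player on sight and plays a melee slash when it reaches them.
; On BeginPlay it attaches a spawned axe to its hand socket and starts a looping random-point patrol.
; PawnSensing raises walk speed and starts the chase, while a retriggerable delay restores patrol and slower speed once sightings stop.
; A flag and DoOnce block repeat attacks until the montage ends.
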(event OnSeePawn(PawnSensing)
  (params (Pawn :type Pawn%20Object%20Reference))
  ;[0 0 0] Chase System
  (Variables|Default|SetCanAttack true)
  (Utilities|FlowControl|Sequence
    (:then_0
      (Variables|/Script/Engine.CharacterMovementComponent|SetMaxWalkSpeed (Variables|Character|GetCharacterMovement) 6e+02)
      (AI|AIMoveTo self "0, 0, 0" (Game|GetPlayerCharacter 0) 7e+01 false
        (:OnSuccess
          (if (Variables|Default|GetCanAttack)
            (Variables|Default|SetCanAttack false)
            (CallFunction|Attack)))))
    (:then_1
      (Utilities|FlowControl|RetriggerableDelay 1.0)
      (CallFunction|SkeletonRoam)
      (Variables|/Script/Engine.CharacterMovementComponent|SetMaxWalkSpeed (Variables|Character|GetCharacterMovement) 3e+02))))

(event Custom|SkeletonRoam
  ;[0 0 0] Patrol System
  (AI|AIMoveTo self (.RandomLocation (AI|Navigation|GetRandomReachablePointinRadius (Transformation|GetActorLocation) 1e+03 0 0)) 0 5.0 false
    (:OnSuccess
      (Utilities|FlowControl|Delay 2.0)
      (CallFunction|SkeletonRoam))))

(event Custom|Attack
  (Utilities|FlowControl|DoOnce false :!label _label
    (:Completed
      (bind _returnvalue (Animation|PlayAnimMontage "/Game/Blueprints/Enemy/Animations/Skeleton_Warrior_Anim_1H_Melee_Attack_Slice_Diagonal_Montage.Skeleton_Warrior_Anim_1H_Melee_Attack_Slice_Diagonal_Montage" 1.0 "None"))
      (Utilities|FlowControl|Delay _returnvalue)
      (Variables|Default|SetCanAttack true)
      (goto _label Reset))))

(event EventBeginPlay
  ;[0 0 0] Attach Sword To Enemy
  (CallFunction|SkeletonRoam)
  (bind _returnvalue (Game|SpawnActorfromClass "/Game/Blueprints/Enemy/BP_EnemAxe.BP_EnemAxe_C" (Transformation|GetSocketTransform (Variables|Character|GetMesh) "hand_r_Weapon_socket" "RTS_World") "Undefined" "MultiplyWithRoot" 0 0))
  (Transformation|AttachComponentToComponent _returnvalue (Variables|Character|GetMesh) "hand_r_Weapon_socket" "SnapToTarget" "SnapToTarget" "SnapToTarget" true))

(event Collision|EventActorBeginOverlap
  (params (OtherActor :type Actor%20Object%20Reference)))

(event EventTick
  (params (DeltaSeconds :type Float%20%28single-precision%29)))

(fn ConstructionScript)